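; BP_Horse_2 is a horse actor, going by its name, that carries a Rat component whose visibility follows a game-wide flag.
; From BeginPlay it polls RatVisible on the BP_full_range_val game instance through a short Delay loop, then hides Rat once the flag is false, with no path to show it again.
; GetLocation exposes the world location of StaticMesh2.
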(event `self.ReceiveBeginPlay`
  (bind _asbp_full_range_val (cast `/Game/Blueprints/BP_full_range_val` (`GameplayStatics.GetGameInstance`)))
  (if (`/Game/Blueprints/BP_full_range_val.rat_visible` _asbp_full_range_val) :!label _label
    (`KismetSystemLibrary.Delay` 0.1)
    (goto _label)
    (else
      (`SceneComponent.SetVisibility` (`self.rat`) false false))))

(fn `get_location`
  (returns (Location :type "Vector Structure"))
  (return (`SceneComponent.K2_GetComponentLocation` (`self.StaticMesh2`))))

(fn `UserConstructionScript`
  (`parent.UserConstructionScript`))