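; BP_GamePlay_Actor runs the policy economy of a plague-management game and registers itself in the BP_full_range_val game instance.
; BeginPlay seeds Policy Points and their growth, which a delayed Tick adds every 30 seconds.
; Button in/out events adjust points, growth and DB through ComsumePolicy, some also toggling policy flags.
; Save copies the "xxx" save_test slot into the named save, but SaveGroup1 and SaveGroup2 items are left unwired.
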(event `self.ReceiveBeginPlay`
  ;[1 1 1] 设置初始Policy Point
  (`KismetSystemLibrary.Delay` 0.2)
  (bind _asbp_full_range_val (cast `/Game/Blueprints/BP_full_range_val` (`GameplayStatics.GetGameInstance`)))
  (set `/Game/Blueprints/BP_full_range_val.policy_point` 80.0 _asbp_full_range_val)
  (set `/Game/Blueprints/BP_full_range_val.increase speed` 15.0 _asbp_full_range_val) ; 该值为每秒增加/减少 IS点Policy_Point
  (bind _asbp_full_range_val_2 (cast `/Game/Blueprints/BP_full_range_val` (`GameplayStatics.GetGameInstance`)))
  (set `/Game/Blueprints/BP_full_range_val.GameActor` self _asbp_full_range_val_2))

(event `self.ReceiveTick`
  (params (DeltaSeconds :type "Float (single-precision)"))
  ;[1 1 1] 设置Policy Point 增量
  (bind _asbp_full_range_val (cast `/Game/Blueprints/BP_full_range_val` (`GameplayStatics.GetGameInstance`)))
  (`KismetSystemLibrary.Delay` 30.0)
  (set `/Game/Blueprints/BP_full_range_val.policy_point` (+ (`/Game/Blueprints/BP_full_range_val.policy_point` _asbp_full_range_val) (`/Game/Blueprints/BP_full_range_val.increase speed` _asbp_full_range_val)) _asbp_full_range_val))

(event `policy_btn_in00`
  (`self.comsume_policy` 10.0 2.0 1))

(event `policy_btn_out00`
  (`self.comsume_policy` 0.0 -2.0 -1))

(event `policy_btn_in01`
  (`self.comsume_policy` 30.0 5.0 3)
  (bind _output_get (set `self.education_active` true))
  (bind _asbp_full_range_val (cast `/Game/Blueprints/BP_full_range_val` (`GameplayStatics.GetGameInstance`)))
  (set `/Game/Blueprints/BP_full_range_val.StrongManagement` _output_get _asbp_full_range_val))

(event `policy_btn_out01`
  (`self.comsume_policy` 0.0 -5.0 -3)
  (bind _output_get (set `self.education_active` false))
  (bind _asbp_full_range_val (cast `/Game/Blueprints/BP_full_range_val` (`GameplayStatics.GetGameInstance`)))
  (set `/Game/Blueprints/BP_full_range_val.StrongManagement` _output_get _asbp_full_range_val))

(event `policy_btn_in02`
  (`self.comsume_policy` 5.0 1.0))

(event `policy_btn_out02`
  (`self.comsume_policy` 0.0 -1.0))

(event `policy_btn_in10`
  (`self.comsume_policy` 20.0 2.5 1))

(event `policy_btn_out10`
  (`self.comsume_policy` 0.0 -2.5 -1))

(event `policy_btn_in11`
  (`self.comsume_policy` 20.0 5.0 2))

(event `policy_btn_out11`
  (`self.comsume_policy` 0.0 -5.0 -2))

(event `policy_btn_in12`
  (`self.comsume_policy` 9999.0 999.0 999))

(event `policy_btn_out12`
  (`self.comsume_policy` 0.0 999.0 999))

(event `policy_btn_out32`)

(event `policy_btn_out42`)

(event `policy_btn_in20`
  (`self.comsume_policy` -20.0 -5.0 -2))

(event `policy_btn_out20`
  (`self.comsume_policy` 0.0 5.0 -2))

(event `policy_btn_in21`
  (`self.comsume_policy` 30.0)
  (bind _output_get (set `self.isolation_active` true))
  (bind _asbp_full_range_val (cast `/Game/Blueprints/BP_full_range_val` (`GameplayStatics.GetGameInstance`)))
  (set `/Game/Blueprints/BP_full_range_val.IsolatedzoneIsvalid` _output_get _asbp_full_range_val))

(event `policy_btn_out21`
  (`self.comsume_policy` 0.0)
  (bind _output_get (set `self.isolation_active` false))
  (bind _asbp_full_range_val (cast `/Game/Blueprints/BP_full_range_val` (`GameplayStatics.GetGameInstance`)))
  (set `/Game/Blueprints/BP_full_range_val.IsolatedzoneIsvalid` _output_get _asbp_full_range_val))

(event `policy_btn_in22`
  (`self.comsume_policy` -20.0 -20.0 -5))

(event `policy_btn_out52`)

(event `policy_btn_out22`
  (`self.comsume_policy` 0.0 20.0 5))

(event `policy_btn_out60`)

(event `policy_btn_in30`
  (`self.comsume_policy` 50.0 30.0)
  (bind _output_get (set `self.cat_active` true))
  (bind _asbp_full_range_val (cast `/Game/Blueprints/BP_full_range_val` (`GameplayStatics.GetGameInstance`)))
  (set `/Game/Blueprints/BP_full_range_val.cat_active` _output_get _asbp_full_range_val))

(event `policy_btn_out30`
  (`self.comsume_policy` 0.0 -30.0)
  (bind _output_get (set `self.cat_active` false))
  (bind _asbp_full_range_val (cast `/Game/Blueprints/BP_full_range_val` (`GameplayStatics.GetGameInstance`)))
  (set `/Game/Blueprints/BP_full_range_val.cat_active` _output_get _asbp_full_range_val))

(event `policy_btn_in31`
  (`self.comsume_policy` 20.0 10.0)
  (bind _output_get (set `self.corpsbury_active` true))
  (bind _asbp_full_range_val (cast `/Game/Blueprints/BP_full_range_val` (`GameplayStatics.GetGameInstance`)))
  (set `/Game/Blueprints/BP_full_range_val.corpsbury_active` _output_get _asbp_full_range_val))

(event `policy_btn_out31`
  (`self.comsume_policy` 0.0 -10.0)
  (bind _output_get (set `self.corpsbury_active` false))
  (bind _asbp_full_range_val (cast `/Game/Blueprints/BP_full_range_val` (`GameplayStatics.GetGameInstance`)))
  (set `/Game/Blueprints/BP_full_range_val.corpsbury_active` _output_get _asbp_full_range_val))

(event `policy_btn_out62`)

(event `policy_btn_in32`)

(event `policy_btn_in40`
  (`self.comsume_policy` 20.0 5.0))

(event `policy_btn_out40`
  (`self.comsume_policy` 0.0 -5.0))

(event `policy_btn_out70`)

(event `policy_btn_in42`)

(event `policy_btn_out72`)

(event `policy_btn_in41`
  (`self.comsume_policy` 10.0 5.0)
  (bind _output_get (set `self.killmission_active` true))
  (bind _asbp_full_range_val (cast `/Game/Blueprints/BP_full_range_val` (`GameplayStatics.GetGameInstance`)))
  (set `/Game/Blueprints/BP_full_range_val.killmission_active` _output_get _asbp_full_range_val))

(event `policy_btn_out41`
  (`self.comsume_policy` 0.0 -5.0)
  (bind _output_get (set `self.killmission_active` false))
  (bind _asbp_full_range_val (cast `/Game/Blueprints/BP_full_range_val` (`GameplayStatics.GetGameInstance`)))
  (set `/Game/Blueprints/BP_full_range_val.killmission_active` _output_get _asbp_full_range_val))

(event `policy_btn_in52`)

(event `policy_btn_in50`
  (`self.comsume_policy` 20.0 -3.0)
  (bind _output_get (set `self.church_active` true))
  (bind _asbp_full_range_val (cast `/Game/Blueprints/BP_full_range_val` (`GameplayStatics.GetGameInstance`)))
  (set `/Game/Blueprints/BP_full_range_val.church_active` _output_get _asbp_full_range_val))

(event `policy_btn_out50`
  (`self.comsume_policy` 0.0 3.0)
  (bind _output_get (set `self.church_active` false))
  (bind _asbp_full_range_val (cast `/Game/Blueprints/BP_full_range_val` (`GameplayStatics.GetGameInstance`)))
  (set `/Game/Blueprints/BP_full_range_val.church_active` _output_get _asbp_full_range_val))

(event `policy_btn_in60`)

(event `policy_btn_in51`
  (`self.comsume_policy` 20.0 20.0)
  (bind _output_get (set `self.town_lockdown_active` true))
  (bind _asbp_full_range_val (cast `/Game/Blueprints/BP_full_range_val` (`GameplayStatics.GetGameInstance`)))
  (set `/Game/Blueprints/BP_full_range_val.town_lockdown_active` _output_get _asbp_full_range_val))

(event `policy_btn_out51`
  (`self.comsume_policy` 0.0 -200.0)
  (bind _output_get (set `self.town_lockdown_active` false))
  (bind _asbp_full_range_val (cast `/Game/Blueprints/BP_full_range_val` (`GameplayStatics.GetGameInstance`)))
  (set `/Game/Blueprints/BP_full_range_val.town_lockdown_active` _output_get _asbp_full_range_val))

(event `policy_btn_in62`)

(event `policy_btn_in70`)

(event `policy_btn_in61`
  (`self.comsume_policy` 9999.0 999.0 999)
  (bind _output_get (set `self.mousein_active` true))
  (bind _asbp_full_range_val (cast `/Game/Blueprints/BP_full_range_val` (`GameplayStatics.GetGameInstance`)))
  (set `/Game/Blueprints/BP_full_range_val.mousein_active` _output_get _asbp_full_range_val))

(event `policy_btn_out61`
  (`self.comsume_policy` 0.0 -999.0 -999)
  (bind _output_get (set `self.mousein_active` false))
  (bind _asbp_full_range_val (cast `/Game/Blueprints/BP_full_range_val` (`GameplayStatics.GetGameInstance`)))
  (set `/Game/Blueprints/BP_full_range_val.mousein_active` _output_get _asbp_full_range_val))

(event `policy_btn_in72`)

(event `policy_btn_in71`
  (`self.comsume_policy` 20.0 5.0 1))

(event `policy_btn_out71`
  (`self.comsume_policy` 0.0 -5.0 -1))

(fn `comsume_policy`
  (params (PP_cost :type "Float (double-precision)") (PP_cost_sustain :type "Float (double-precision)") (DB :type Integer))
  (bind _asbp_full_range_val (cast `/Game/Blueprints/BP_full_range_val` (`GameplayStatics.GetGameInstance`)))
  (set `/Game/Blueprints/BP_full_range_val.policy_point` (- (`/Game/Blueprints/BP_full_range_val.policy_point` _asbp_full_range_val) PP_cost) _asbp_full_range_val)
  (set `/Game/Blueprints/BP_full_range_val.increase speed` (- (`/Game/Blueprints/BP_full_range_val.increase speed` _asbp_full_range_val) PP_cost_sustain) _asbp_full_range_val)
  (set `/Game/Blueprints/BP_full_range_val.DB` (+ (`/Game/Blueprints/BP_full_range_val.DB` _asbp_full_range_val) DB) _asbp_full_range_val))

(fn `save`
  (bind _asbp_full_range_val (cast `/Game/Blueprints/BP_full_range_val` (`GameplayStatics.GetGameInstance`)))
  (bind _savename (`/Game/Blueprints/BP_full_range_val.savename` _asbp_full_range_val))
  (bind _returnvalue (`GameplayStatics.DoesSaveGameExist` _savename))
  (if _returnvalue
    (bind _returnvalue_2 (`GameplayStatics.LoadGameFromSlot` _savename))
    (bind _assave (cast `/Game/UI/save` _returnvalue_2))
    (bind _returnvalue_3 (`GameplayStatics.LoadGameFromSlot` "xxx"))
    (bind _assave_test (cast `/Game/UI/save_test` _returnvalue_3))
    (set `/Game/UI/save.transform` (`/Game/UI/save_test.transform` _assave_test) _assave)
    (bind _position (`/Game/UI/save.position` _assave))
    (for (_ _array_index) _position
      (`KismetArrayLibrary.Array_Set` _position _array_index (`|GetArrayItem` (`/Game/UI/save_test.position` _assave_test) _array_index) true))
    (bind _save_virus_status (`/Game/UI/save.save_virus_status` _assave))
    (for (_ _array_index_2) _save_virus_status
      (`KismetArrayLibrary.Array_Set` _save_virus_status _array_index_2 (`|GetArrayItem` (`/Game/UI/save_test.save_virus_status` _assave_test) _array_index_2) true))
    (set `/Game/UI/save.save_DB` (`/Game/UI/save_test.save_DB` _assave_test) _assave)
    (set `/Game/UI/save.save_policy_point` (`/Game/UI/save_test.save_policy_point` _assave_test) _assave)
    (set `/Game/UI/save.save_increase speed` (`/Game/UI/save_test.save_increase speed` _assave_test) _assave)
    (set `/Game/UI/save.save_StrongManagement` (`/Game/UI/save_test.save_StrongManagement` _assave_test) _assave)
    (set `/Game/UI/save.save_StrongIsolated` (`/Game/UI/save_test.save_StrongIsolated` _assave_test) _assave)
    (set `/Game/UI/save.save_IsolatedzoneIsvalid` (`/Game/UI/save_test.save_IsolatedzoneIsvalid` _assave_test) _assave)
    (set `/Game/UI/save.save_education_active` (`/Game/UI/save_test.save_education_active` _assave_test) _assave)
    (set `/Game/UI/save.save_cat_active` (`/Game/UI/save_test.save_cat_active` _assave_test) _assave)
    (set `/Game/UI/save.save_corpsbury_active` (`/Game/UI/save_test.save_corpsbury_active` _assave_test) _assave)
    (set `/Game/UI/save.save_killmission_active` (`/Game/UI/save_test.save_killmission_active` _assave_test) _assave)
    (set `/Game/UI/save.save_GameActor` (`/Game/UI/save_test.save_GameActor` _assave_test) _assave)
    (set `/Game/UI/save.save_church_active` (`/Game/UI/save_test.save_church_active` _assave_test) _assave)
    (set `/Game/UI/save.save_town_lockdown_active` (`/Game/UI/save_test.save_town_lockdown_active` _assave_test) _assave)
    (set `/Game/UI/save.save_mousein_active` (`/Game/UI/save_test.save_mousein_active` _assave_test) _assave)
    (set `/Game/UI/save.save_Isolation_active` (`/Game/UI/save_test.save_Isolation_active` _assave_test) _assave)
    (set `/Game/UI/save.save_People_Num` (`/Game/UI/save_test.save_People_Num` _assave_test) _assave)
    (bind _save_people_transport (`/Game/UI/save.save_People_Transport` _assave))
    (for (_ _array_index_3) _save_people_transport
      (`KismetArrayLibrary.Array_Set` _save_people_transport _array_index_3 (`|GetArrayItem` (`/Game/UI/save_test.save_People_Transport` _assave_test) _array_index_3) true))
    (set `/Game/UI/save.save_Hour` (`/Game/UI/save_test.save_Hour` _assave_test) _assave)
    (set `/Game/UI/save.save_Day` (`/Game/UI/save_test.save_Day` _assave_test) _assave)
    (set `/Game/UI/save.save_Daycount` (`/Game/UI/save_test.save_Daycount` _assave_test) _assave)
    (bind _save_message (`/Game/UI/save.save_message` _assave))
    (for (_ _array_index_4) _save_message
      (`KismetArrayLibrary.Array_Set` _save_message _array_index_4 (`|GetArrayItem` (`/Game/UI/save_test.save_message` _assave_test) _array_index_4) true))
    (bind _save_group_0 (`/Game/UI/save.save_group_0` _assave))
    (for (_ _array_index_5) _save_group_0
      (`KismetArrayLibrary.Array_Set` _save_group_0 _array_index_5 (`|GetArrayItem` (`/Game/UI/save_test.save_group_0` _assave_test) _array_index_5) true))
    (set `/Game/UI/save.save_array_value` (`/Game/UI/save_test.save_array_value` _assave_test) _assave)
    (bind _save_group_1 (`/Game/UI/save.save_group_1` _assave))
    (for (_ _array_index_6) _save_group_1
      (`KismetArrayLibrary.Array_Set` _save_group_1 _array_index_6 false true))
    (bind _save_group_2 (`/Game/UI/save.save_group_2` _assave))
    (for (_ _array_index_7) _save_group_2
      (`KismetArrayLibrary.Array_Set` _save_group_2 _array_index_7 false true))
    (set `/Game/UI/save.save_if_savegame` (`/Game/UI/save_test.save_if_savegame` _assave_test) _assave)
    (set `/Game/UI/save.save_savename` (`/Game/UI/save_test.save_savename` _assave_test) _assave)
    (set `/Game/UI/save.save_middle_point` (`/Game/UI/save_test.save_middle_point` _assave_test) _assave)
    (bind _returnvalue_4 (`GameplayStatics.SaveGameToSlot` _assave _savename))
    (if _returnvalue_4
      (`KismetSystemLibrary.PrintString` "savegamesuccess1"))
    (else
      (bind _returnvalue_5 (`GameplayStatics.CreateSaveGameObject` "/Game/UI/save.save_C"))
      (bind _returnvalue_6 (`GameplayStatics.LoadGameFromSlot` "xxx"))
      (bind _assave_test_2 (cast `/Game/UI/save_test` _returnvalue_6))
      (set `/Game/UI/save.transform` (`/Game/UI/save_test.transform` _assave_test_2) _returnvalue_5)
      (bind _position_2 (`/Game/UI/save.position` _returnvalue_5))
      (for (_ _array_index_8) _position_2
        (`KismetArrayLibrary.Array_Set` _position_2 _array_index_8 (`|GetArrayItem` (`/Game/UI/save_test.position` _assave_test_2) _array_index_8) true))
      (bind _save_virus_status_2 (`/Game/UI/save.save_virus_status` _returnvalue_5))
      (for (_ _array_index_9) _save_virus_status_2
        (`KismetArrayLibrary.Array_Set` _save_virus_status_2 _array_index_9 (`|GetArrayItem` (`/Game/UI/save_test.save_virus_status` _assave_test_2) _array_index_9) true))
      (set `/Game/UI/save.save_DB` (`/Game/UI/save_test.save_DB` _assave_test_2) _returnvalue_5)
      (set `/Game/UI/save.save_policy_point` (`/Game/UI/save_test.save_policy_point` _assave_test_2) _returnvalue_5)
      (set `/Game/UI/save.save_increase speed` (`/Game/UI/save_test.save_increase speed` _assave_test_2) _returnvalue_5)
      (set `/Game/UI/save.save_StrongManagement` (`/Game/UI/save_test.save_StrongManagement` _assave_test_2) _returnvalue_5)
      (set `/Game/UI/save.save_StrongIsolated` (`/Game/UI/save_test.save_StrongIsolated` _assave_test_2) _returnvalue_5)
      (set `/Game/UI/save.save_IsolatedzoneIsvalid` (`/Game/UI/save_test.save_IsolatedzoneIsvalid` _assave_test_2) _returnvalue_5)
      (set `/Game/UI/save.save_education_active` (`/Game/UI/save_test.save_education_active` _assave_test_2) _returnvalue_5)
      (set `/Game/UI/save.save_cat_active` (`/Game/UI/save_test.save_cat_active` _assave_test_2) _returnvalue_5)
      (set `/Game/UI/save.save_corpsbury_active` (`/Game/UI/save_test.save_corpsbury_active` _assave_test_2) _returnvalue_5)
      (set `/Game/UI/save.save_killmission_active` (`/Game/UI/save_test.save_killmission_active` _assave_test_2) _returnvalue_5)
      (set `/Game/UI/save.save_GameActor` (`/Game/UI/save_test.save_GameActor` _assave_test_2) _returnvalue_5)
      (set `/Game/UI/save.save_church_active` (`/Game/UI/save_test.save_church_active` _assave_test_2) _returnvalue_5)
      (set `/Game/UI/save.save_town_lockdown_active` (`/Game/UI/save_test.save_town_lockdown_active` _assave_test_2) _returnvalue_5)
      (set `/Game/UI/save.save_mousein_active` (`/Game/UI/save_test.save_mousein_active` _assave_test_2) _returnvalue_5)
      (set `/Game/UI/save.save_Isolation_active` (`/Game/UI/save_test.save_Isolation_active` _assave_test_2) _returnvalue_5)
      (set `/Game/UI/save.save_People_Num` (`/Game/UI/save_test.save_People_Num` _assave_test_2) _returnvalue_5)
      (bind _save_people_transport_2 (`/Game/UI/save.save_People_Transport` _returnvalue_5))
      (for (_ _array_index_10) _save_people_transport_2
        (`KismetArrayLibrary.Array_Set` _save_people_transport_2 _array_index_10 (`|GetArrayItem` (`/Game/UI/save_test.save_People_Transport` _assave_test_2) _array_index_10) true))
      (set `/Game/UI/save.save_Hour` (`/Game/UI/save_test.save_Hour` _assave_test_2) _returnvalue_5)
      (set `/Game/UI/save.save_Day` (`/Game/UI/save_test.save_Day` _assave_test_2) _returnvalue_5)
      (set `/Game/UI/save.save_Daycount` (`/Game/UI/save_test.save_Daycount` _assave_test_2) _returnvalue_5)
      (bind _save_message_2 (`/Game/UI/save.save_message` _returnvalue_5))
      (for (_ _array_index_11) _save_message_2
        (`KismetArrayLibrary.Array_Set` _save_message_2 _array_index_11 (`|GetArrayItem` (`/Game/UI/save_test.save_message` _assave_test_2) _array_index_11) true))
      (bind _save_group_0_2 (`/Game/UI/save.save_group_0` _returnvalue_5))
      (for (_ _array_index_12) _save_group_0_2
        (`KismetArrayLibrary.Array_Set` _save_group_0_2 _array_index_12 (`|GetArrayItem` (`/Game/UI/save_test.save_group_0` _assave_test_2) _array_index_12) true))
      (set `/Game/UI/save.save_array_value` (`/Game/UI/save_test.save_array_value` _assave_test_2) _returnvalue_5)
      (bind _save_group_1_2 (`/Game/UI/save.save_group_1` _returnvalue_5))
      (for (_ _array_index_13) _save_group_1_2
        (`KismetArrayLibrary.Array_Set` _save_group_1_2 _array_index_13 false true))
      (bind _save_group_2_2 (`/Game/UI/save.save_group_2` _returnvalue_5))
      (for (_ _array_index_14) _save_group_2_2
        (`KismetArrayLibrary.Array_Set` _save_group_2_2 _array_index_14 false true))
      (set `/Game/UI/save.save_if_savegame` (`/Game/UI/save_test.save_if_savegame` _assave_test_2) _returnvalue_5)
      (set `/Game/UI/save.save_savename` (`/Game/UI/save_test.save_savename` _assave_test_2) _returnvalue_5)
      (set `/Game/UI/save.save_middle_point` (`/Game/UI/save_test.save_middle_point` _assave_test_2) _returnvalue_5)
      (bind _returnvalue_7 (`GameplayStatics.SaveGameToSlot` _returnvalue_5 _savename))
      (if _returnvalue_7
        (`KismetSystemLibrary.PrintString` "savegamesuccess2")))))

(fn `UserConstructionScript`)