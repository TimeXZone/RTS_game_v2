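; NPC character that carries, spreads and suffers from a virus in an epidemic simulation.
; Three scaled overlap boxes (near, mid, far) on infected NPCs flag others as exposed.
; Delayed Tick branches make graded percentage rolls, biased by distance or game-instance values, to change InfectStatus and decide death.
; Severe cases immobilise people, and infected people join the game instance's isolation transport queue, at a lower threshold under strong isolation.
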(event `self.ReceiveBeginPlay`
  ;[1 1 1] 初始化人物
  (`self.vir_bio_init` 20.0 80.0 60.0 40.0 5.0)
  (set `self.infect_radius` 5.0))

(event `self.ReceiveTick`
  (params (DeltaSeconds :type "Float (single-precision)"))
  (bind _infect_status (`self.infect_status`))
  (bind _infect_status_2 (`self.infect_status`))
  (`|ExecutionSequence`
    (:`then_0`
      (`KismetSystemLibrary.Delay` 5.0)
      (bind (_infect_radius_near _infect_radius_mid _infect_radius_far) (`self.infect_radius_to_3`))
      ;[1 1 1] 初始化人物
      (`SceneComponent.SetWorldScale3D` (`self.Infect_box_near`) _infect_radius_near)
      (`SceneComponent.SetWorldScale3D` (`self.Infect_box_mid`) _infect_radius_mid)
      (`SceneComponent.SetWorldScale3D` (`self.Infect_box_far`) _infect_radius_far))
    (:`then_1`
      (`KismetSystemLibrary.Delay` 300.0)
      ;[1 1 1] 病重分支
      (if (>= (`self.infect_status`) 1)
        (bind (_time_worsen _death_percent _heavy_percent) (`self.show_npc_state`))
        (bind _returnvalue (`self.check_func` _heavy_percent (`/Game/Blueprints/BP_full_range_val.DB` (stale _asbp_full_range_val))))
        (bind (_success _huge_success _fail _huge_fail) (`self.switch_func` _returnvalue))
        (`|ExecutionSequence`
          (:`then_0`
            (if _success
              (set `self.infect_status` (+ (`self.infect_status`) 1))))
          (:`then_1`
            (if _huge_success
              (set `self.infect_status` (+ (`self.infect_status`) 2))))
          (:`then_2`
            (if _fail
              (set `self.infect_status` (+ (`self.infect_status`) 0))))
          (:`then_3`
            (if _huge_fail
              (set `self.infect_status` (+ (`self.infect_status`) -1)))))))
    (:`then_2`
      (`KismetSystemLibrary.Delay` 60.0)
      ;[1 1 1] 感染
      (`|ExecutionSequence`
        (:`then_0`
          (if (`self.whether_would_be_infect_near`)
            (bind (_time_worsen_2 _death_percent_2 _heavy_percent_2 _infect_percent) (`self.show_npc_state`))
            (bind _returnvalue_2 (`self.check_func` _infect_percent 1))
            (bind (_success_2 _huge_success_2 _fail_2 _huge_fail_2) (`self.switch_func` _returnvalue_2))
            (`|ExecutionSequence`
              (:`then_0`
                (if _success_2
                  (set `self.infect_status` (+ (`self.infect_status`) 1))))
              (:`then_1`
                (if _huge_success_2
                  (set `self.infect_status` (+ (`self.infect_status`) 2))))
              (:`then_2`
                (if _fail_2
                  (set `self.infect_status` (+ (`self.infect_status`) 0))))
              (:`then_3`
                (if _huge_fail_2
                  (set `self.infect_status` (+ (`self.infect_status`) -1)))))))
        (:`then_1`
          (if (`self.whether_would_be_infect_mid`)
            (bind (_time_worsen_3 _death_percent_3 _heavy_percent_3 _infect_percent_2) (`self.show_npc_state`))
            (bind _returnvalue_3 (`self.check_func` _infect_percent_2))
            (bind (_success_3 _huge_success_3 _fail_3 _huge_fail_3) (`self.switch_func` _returnvalue_3))
            (`|ExecutionSequence`
              (:`then_0`
                (if _success_3
                  (set `self.infect_status` (+ (`self.infect_status`) 1))))
              (:`then_1`
                (if _huge_success_3
                  (set `self.infect_status` (+ (`self.infect_status`) 2))))
              (:`then_2`
                (if _fail_3
                  (set `self.infect_status` (+ (`self.infect_status`) 0))))
              (:`then_3`
                (if _huge_fail_3
                  (set `self.infect_status` (+ (`self.infect_status`) -1)))))))
        (:`then_2`
          (if (`self.whether_would_be_infect_far`)
            (bind (_time_worsen_4 _death_percent_4 _heavy_percent_4 _infect_percent_3) (`self.show_npc_state`))
            (bind _returnvalue_4 (`self.check_func` _infect_percent_3 -1))
            (bind (_success_4 _huge_success_4 _fail_4 _huge_fail_4) (`self.switch_func` _returnvalue_4))
            (`|ExecutionSequence`
              (:`then_0`
                (if _success_4
                  (set `self.infect_status` (+ (`self.infect_status`) 1))))
              (:`then_1`
                (if _huge_success_4
                  (set `self.infect_status` (+ (`self.infect_status`) 2))))
              (:`then_2`
                (if _fail_4
                  (set `self.infect_status` (+ (`self.infect_status`) 0))))
              (:`then_3`
                (if _huge_fail_4
                  (set `self.infect_status` (+ (`self.infect_status`) -1)))))))))
    (:`then_3`
      (if (>= (`self.infect_status`) 3)
        (if (`self.isPeople`)
          (set `self.isdown` true)
          (`ActorComponent.Deactivate` (`self.CharacterMovement`)))
        (else
          (set `self.isdown` false))))
    (:`then_4`
      (bind _asbp_full_range_val (cast `/Game/Blueprints/BP_full_range_val` (`GameplayStatics.GetGameInstance`))))
    (:`then_5`
      ;[1 1 1] 死亡判定
      (if (`self.undeath`)
        _
        (elif (`self.dead_sgn`)
          _
          (elif (>= _infect_status 4)
            (`KismetSystemLibrary.Delay` 10.0)
            (bind (_time_worsen_5 _death_percent_5) (`self.show_npc_state`))
            (bind _returnvalue_5 (`self.check_func` _death_percent_5 (- _infect_status 4)))
            (set `self.dead_sgn` (<= _returnvalue_5 1))))))
    (:`then_6`
      (bind _asbp_full_range_val_2 (cast `/Game/Blueprints/BP_full_range_val` (`GameplayStatics.GetGameInstance`)))
      ;[1 1 1] 是否启用加强隔离
      (if (`/Game/Blueprints/BP_full_range_val.StrongIsolated` _asbp_full_range_val_2)
        (if (not (< _infect_status_2 1))
          (if (`self.isPeople`) :!label _label
            ;[1 1 1] inLine表示此人在队列中
            (if (not (`self.inLine`))
              ;[1 1 1] isIsolated表示此人在隔离区，若在隔离区，不需要运送
              (if (`self.isolated`)
                _
                (elif (not (`self.dead_sgn`))
                  (bind _asbp_full_range_val_3 (cast `/Game/Blueprints/BP_full_range_val` (`GameplayStatics.GetGameInstance`)))
                  (`KismetArrayLibrary.Array_Add` (`/Game/Blueprints/BP_full_range_val.People_Transport` _asbp_full_range_val_3) self)
                  (set `self.inLine` true))))))
        (elif (not (<= _infect_status_2 1))
          (goto _label))))))

(event `self.Infect_box_near.OnComponentBeginOverlap`
  (params (OverlappedComponent :type "PrimitiveComponent Object Reference") (OtherActor :type "Actor Object Reference") (OtherComp :type "PrimitiveComponent Object Reference") (OtherBodyIndex :type Integer) (bFromSweep :type Boolean) (SweepResult :type "HitResult Structure (by ref)"))
  ;[1 1 1] 感染
  (bind _asbp_my_npc_character_with_virus (cast `/Game/Blueprints/BP_MyNPC_character_with_virus` OtherActor))
  (if (>= (`self.infect_status`) 1)
    (set `/Game/Blueprints/BP_MyNPC_character_with_virus.whether_would_be_infect_near` true _asbp_my_npc_character_with_virus)))

(event `self.Infect_box_near.OnComponentEndOverlap`
  (params (OverlappedComponent :type "PrimitiveComponent Object Reference") (OtherActor :type "Actor Object Reference") (OtherComp :type "PrimitiveComponent Object Reference") (OtherBodyIndex :type Integer))
  ;[1 1 1] 感染
  (bind _asbp_my_npc_character_with_virus (cast `/Game/Blueprints/BP_MyNPC_character_with_virus` OtherActor))
  (set `/Game/Blueprints/BP_MyNPC_character_with_virus.whether_would_be_infect_near` false _asbp_my_npc_character_with_virus))

(event `self.Infect_box_mid.OnComponentBeginOverlap`
  (params (OverlappedComponent :type "PrimitiveComponent Object Reference") (OtherActor :type "Actor Object Reference") (OtherComp :type "PrimitiveComponent Object Reference") (OtherBodyIndex :type Integer) (bFromSweep :type Boolean) (SweepResult :type "HitResult Structure (by ref)"))
  ;[1 1 1] 感染
  (bind _asbp_my_npc_character_with_virus (cast `/Game/Blueprints/BP_MyNPC_character_with_virus` OtherActor))
  (if (>= (`self.infect_status`) 1)
    (set `/Game/Blueprints/BP_MyNPC_character_with_virus.whether_would_be_infect_mid` true _asbp_my_npc_character_with_virus)))

(event `self.Infect_box_mid.OnComponentEndOverlap`
  (params (OverlappedComponent :type "PrimitiveComponent Object Reference") (OtherActor :type "Actor Object Reference") (OtherComp :type "PrimitiveComponent Object Reference") (OtherBodyIndex :type Integer))
  ;[1 1 1] 感染
  (bind _asbp_my_npc_character_with_virus (cast `/Game/Blueprints/BP_MyNPC_character_with_virus` OtherActor))
  (set `/Game/Blueprints/BP_MyNPC_character_with_virus.whether_would_be_infect_mid` false _asbp_my_npc_character_with_virus))

(event `self.Infect_box_far.OnComponentBeginOverlap`
  (params (OverlappedComponent :type "PrimitiveComponent Object Reference") (OtherActor :type "Actor Object Reference") (OtherComp :type "PrimitiveComponent Object Reference") (OtherBodyIndex :type Integer) (bFromSweep :type Boolean) (SweepResult :type "HitResult Structure (by ref)"))
  ;[1 1 1] 感染
  (bind _asbp_my_npc_character_with_virus (cast `/Game/Blueprints/BP_MyNPC_character_with_virus` OtherActor))
  (if (>= (`self.infect_status`) 1)
    (set `/Game/Blueprints/BP_MyNPC_character_with_virus.whether_would_be_infect_far` true _asbp_my_npc_character_with_virus)))

(event `self.Infect_box_far.OnComponentEndOverlap`
  (params (OverlappedComponent :type "PrimitiveComponent Object Reference") (OtherActor :type "Actor Object Reference") (OtherComp :type "PrimitiveComponent Object Reference") (OtherBodyIndex :type Integer))
  ;[1 1 1] 感染
  (bind _asbp_my_npc_character_with_virus (cast `/Game/Blueprints/BP_MyNPC_character_with_virus` OtherActor))
  (set `/Game/Blueprints/BP_MyNPC_character_with_virus.whether_would_be_infect_far` false _asbp_my_npc_character_with_virus))

(fn `infect_radius_to_3`
  (returns (infect_radius_near :type "Vector Structure") (infect_radius_mid :type "Vector Structure") (infect_radius_far :type "Vector Structure"))
  (bind _infect_radius (`self.infect_radius`))
  (bind _returnvalue (* _infect_radius 2.0))
  (bind _returnvalue_2 (* _infect_radius 0.25))
  (return (`KismetMathLibrary.MakeVector` _returnvalue_2 _returnvalue_2 _returnvalue_2) (`KismetMathLibrary.MakeVector` _infect_radius _infect_radius _infect_radius) (`KismetMathLibrary.MakeVector` _returnvalue _returnvalue _returnvalue)))

(fn `UserConstructionScript`)