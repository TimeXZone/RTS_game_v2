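; BP_Camera is a free-moving camera actor driven by player input axes.
; MoveForward and MoveRight offset it along its forward and right vectors at a fixed step per axis update, without sweep or delta-time scaling.
; UpDown applies pitch as a local rotation and LeftRight applies yaw as a world rotation, so looking around does not accumulate roll.
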(event `InputAxis|MoveForward`
  (params (AxisValue :type "Float (single-precision)"))
  ;[1 1 1] 相机前后左右位置变换
  (`self.K2_AddActorWorldOffset` (* (`self.GetActorForwardVector`) (* (`self.GetInputAxisValue`) 10.0))))

(event `InputAxis|UpDown`
  (params (AxisValue :type "Float (single-precision)"))
  (`self.K2_AddActorLocalRotation` (`KismetMathLibrary.MakeRotator` 0.0 (`self.GetInputAxisValue`))))

(event `InputAxis|MoveRight`
  (params (AxisValue :type "Float (single-precision)"))
  ;[1 1 1] 相机前后左右位置变换
  (`self.K2_AddActorWorldOffset` (* (`self.GetActorRightVector`) (* (`self.GetInputAxisValue`) 10.0))))

(event `InputAxis|LeftRight`
  (params (AxisValue :type "Float (single-precision)"))
  (`self.K2_AddActorWorldRotation` (`KismetMathLibrary.MakeRotator` 0.0 0.0 (`self.GetInputAxisValue`))))

(fn `UserConstructionScript`)