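; Player controller that drives the BP_CameraPawn with screen-edge panning and right-button rotation.
; While the right button is up, mouse axis events apply a fixed local offset from MouseControl_EdgeDrag, which checks cursor position against viewport edges without delta-time scaling.
; While it is held, LeftRight applies world yaw and UpDown applies local pitch.
; Z resets the pawn's rotation to zero.
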(event `self.ReceiveBeginPlay`
  ;[1 1 1] 获取相机Pawn
  (bind _asbp_camera_pawn (cast `/Game/GameMode/BP_CameraPawn` (`GameplayStatics.GetPlayerPawn` 0)))
  (set `self.Ref_cameraPawn` _asbp_camera_pawn))

(event `InputAxis|LeftRight`
  (params (AxisValue :type "Float (single-precision)"))
  ;[1 1 1] 点击右键后移动鼠标或按键盘上下左右进行镜头旋转
  (if (`self.RightClick`)
    (`self.K2_AddActorWorldRotation` (`self.Ref_cameraPawn`) (`KismetMathLibrary.MakeRotator` 0.0 0.0 (* AxisValue -1.0)) false false)))

(event `InputAxisKey|MouseX`
  (params (AxisValue :type "Float (single-precision)"))
  ;[1 1 1] 鼠标在屏幕边缘时，移动窗口
  (if (not (`self.RightClick`))
    (`self.K2_AddActorLocalOffset` (`self.Ref_cameraPawn`) (`self.MouseControl_EdgeDrag` 0.015) false false)))

(event `InputAxisKey|MouseY`
  (params (AxisValue :type "Float (single-precision)"))
  ;[1 1 1] 鼠标在屏幕边缘时，移动窗口
  (if (not (`self.RightClick`))
    (`self.K2_AddActorLocalOffset` (`self.Ref_cameraPawn`) (`self.MouseControl_EdgeDrag` 0.015) false false)))

(event `InputAxis|UpDown`
  (params (AxisValue :type "Float (single-precision)"))
  ;[1 1 1] 点击右键后移动鼠标或按键盘上下左右进行镜头旋转
  (if (`self.RightClick`)
    (`self.K2_AddActorLocalRotation` (`self.Ref_cameraPawn`) (`KismetMathLibrary.MakeRotator` 0.0 (* AxisValue -1.0) 0.0) false false)))

(event `Key|RightMouseButton`
  (params (Key :type "Key Structure"))
  (:`Pressed`
    (set `self.RightClick` true))
  (:`Released`
    (set `self.RightClick` false)))

(event `Key|Z`
  (params (Key :type "Key Structure"))
  ;[1 1 1] 按键盘Z，恢复镜头
  (:`Pressed`
    (`self.K2_SetActorRotation` :`self` (`self.Ref_cameraPawn`))))

(fn `MouseControl_EdgeDrag`
  (params (EdgeSize :type "Float (double-precision)"))
  (returns (Location :type "Vector Structure"))
  (bind _returnvalue (- 1.0 EdgeSize))
  (bind (_sizex _sizey) (`self.GetViewportSize`))
  (bind (_locationx _locationy _returnvalue_2) (`self.GetMousePosition`))
  (bind _returnvalue_3 (/ _locationy (`KismetMathLibrary.Conv_IntToDouble` _sizey)))
  (bind _returnvalue_4 (/ _locationx (`KismetMathLibrary.Conv_IntToDouble` _sizex)))
  (return (`KismetMathLibrary.SelectVector` (+ (+ (`KismetMathLibrary.SelectVector` (0.0 10.0 0.0) (0.0 0.0 0.0) (>= _returnvalue_4 _returnvalue)) (`KismetMathLibrary.SelectVector` (0.0 -10.0 0.0) (0.0 0.0 0.0) (<= _returnvalue_4 EdgeSize))) (+ (`KismetMathLibrary.SelectVector` (-10.0 0.0 0.0) (0.0 0.0 0.0) (>= _returnvalue_3 _returnvalue)) (`KismetMathLibrary.SelectVector` (10.0 0.0 0.0) (0.0 0.0 0.0) (<= _returnvalue_3 EdgeSize)))) (0.0 0.0 0.0) _returnvalue_2)))

(fn `UserConstructionScript`)